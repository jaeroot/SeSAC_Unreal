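; BP_Door1 is a double swinging door with OpenDoor and CloseDoor events and no trigger logic of its own.
; OpenDoor plays a timeline that lerps the relative yaw of both leaf meshes through 90 degrees, with IsFront selecting the swing direction.
; CloseDoor reverses that timeline from its end, so closing always starts from the fully open pose.
; IsFront is only read here, never set.
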(event `self.OpenDoor`
  (bind (_direction `_새_트랙_0`) (`Timeline|타임라인` :!label _label)
    (:`Update`
      (if (`self.bIsFront`)
        (`SceneComponent.K2_SetRelativeRotation` (`self.mMesh1`) (`KismetMathLibrary.MakeRotator` 0.0 0.0 (`KismetMathLibrary.Lerp` 180.0 270.0 `_새_트랙_0`)) false false)
        (`SceneComponent.K2_SetRelativeRotation` (`self.mMesh2`) (`KismetMathLibrary.MakeRotator` 0.0 0.0 (`KismetMathLibrary.Lerp` 0.0 -90.0 `_새_트랙_0`)) false false)
        (else
          (`SceneComponent.K2_SetRelativeRotation` (`self.mMesh1`) (`KismetMathLibrary.MakeRotator` 0.0 0.0 (`KismetMathLibrary.Lerp` 180.0 90.0 `_새_트랙_0`)) false false)
          (`SceneComponent.K2_SetRelativeRotation` (`self.mMesh2`) (`KismetMathLibrary.MakeRotator` 0.0 0.0 (`KismetMathLibrary.Lerp` 0.0 90.0 `_새_트랙_0`)) false false))))))

(event `self.CloseDoor`
  (goto _label :!via `ReverseFromEnd`))

(fn `UserConstructionScript`)